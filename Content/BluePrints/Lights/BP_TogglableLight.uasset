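; BP_TogglableLight is a spot light Blueprint that can be switched on and off.
; ToggleLights flips IsON, sets the SpotLight intensity to a hardcoded bright value or zero, and prints the new state.
; The construction script instead sets SpotLight visibility from IsON, which the toggle never updates, so a light constructed off stays hidden when toggled.
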(event EventToggleLights
  (bind _spotlight (Variables|Default|GetSpotLight))
  (bind _output_get (Variables|Default|SetIsON? (not (Variables|Default|GetIsON?))))
  (if _output_get
    (Rendering|Components|Light|SetIntensity _spotlight 1e+05)
    (Development|PrintString "On")
    (else
      (Rendering|Components|Light|SetIntensity _spotlight 0.0)
      (Development|PrintString "Off"))))

(fn ConstructionScript
  (Rendering|SetVisibility (Variables|Default|GetSpotLight) (Variables|Default|GetIsON?) false))