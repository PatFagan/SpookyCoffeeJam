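; NoteFinal_BP is an interactable note that plays a timed writing sequence and then loads the LV_ColtonTest level.
; Interact toggles reading, hiding the note mesh and locking player move and look input.
; The first pickup runs a DoOnce sequence: note widget, scribble sound, finished-note widget, then FadeOut_BP's fade to black before the level opens.
; NoteRead is set on put-down and routes later pickups to the finished-note widget.
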(event Custom|TogglePickup
  (bind _returnvalue (Game|GetPlayerController 0))
  (bind _returnvalue_2 (Game|GetPlayerController 0))
  (if (Variables|Default|GetIsReading)
    (CallFunction|PutDownNote)
    (Input|SetIgnoreMoveInput _returnvalue_2 false)
    (Input|SetIgnoreLookInput _returnvalue_2 false)
    (Variables|Default|SetNoteRead true)
    (else
      (if (Variables|Default|GetNoteRead)
        (CallFunction|PickupNote)
        (else
          (CallFunction|WriteNote)))
      (Input|SetIgnoreMoveInput _returnvalue true)
      (Input|SetIgnoreLookInput _returnvalue true))))

(event Custom|PickupNote
  (if (Variables|Default|GetNoteRead)
    (UserInterface|Viewport|AddtoViewport (Variables|Default|GetFinalRef) 0)
    (else
      (bind _returnvalue (UserInterface|CreateWidget (Variables|Default|GetWidget)))
      (bind _output_get (Variables|Default|SetWidgetRef _returnvalue))
      (UserInterface|Viewport|AddtoViewport _output_get 0)))
  (Rendering|SetVisibility (Variables|Default|GetNote) false false)
  (Variables|Default|SetIsReading true))

(event Custom|PutDownNote
  (Utilities|IsValid (Variables|Default|GetWidgetRef)
    (:Is%20Valid
      (Widget|RemovefromParent (Variables|Default|GetFinalRef))
      (Rendering|SetVisibility (Variables|Default|GetNote) true false)
      (Variables|Default|SetIsReading false))))

(event Custom|WriteNote
  (Utilities|FlowControl|DoOnce false
    (:Completed
      (Input|DisableInput (Game|GetPlayerController 0))
      (Development|PrintString "Disable")
      (CallFunction|PickupNote)
      (Utilities|FlowControl|Delay 1.0)
      (Widget|RemovefromParent (Variables|Default|GetWidgetRef))
      (Audio|PlaySound2D "/Game/Audio/SFX/Scribble.Scribble" 1.0 1.0 0.0 0 0)
      (Utilities|FlowControl|Delay 2.0)
      (bind _returnvalue (UserInterface|CreateWidget (Variables|Default|GetFinalWidget)))
      (bind _output_get (Variables|Default|SetFinalRef _returnvalue))
      (UserInterface|Viewport|AddtoViewport _output_get 0)
      (Utilities|FlowControl|Delay 2.0)
      (Widget|RemovefromParent (Variables|Default|GetFinalRef))
      (bind _returnvalue_2 (UserInterface|CreateWidget (Variables|Default|GetFadeOut)))
      (bind _output_get_2 (Variables|Default|SetNewVar_0 _returnvalue_2))
      (UserInterface|Viewport|AddtoViewport _returnvalue_2 0)
      (bind _asfade_out_bp (Utilities|Casting|CastToFadeOut_BP (Variables|Default|GetNewVar_0)))
      (Default|FadeinBlack _asfade_out_bp)
      (Utilities|FlowControl|Delay 5.0)
      (Game|OpenLevel(byObjectReference) "/Game/Maps/LV_ColtonTest.LV_ColtonTest")
      (Widget|RemovefromParent (Variables|Default|GetNewVar_0))
      (Input|EnableInput (Game|GetPlayerController 0)))))

(event EventInteract
  (CallFunction|TogglePickup)
  (Development|PrintString "Hello"))

(event Input|KeyboardEvents|AnyKey
  (params (Key :type Key%20Structure :default "None"))
  (:Pressed
    (CallFunction|PutDownNote)))

(fn ConstructionScript)