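; BP_ElectricalSwitch is an interactable switch in a puzzle to charge the electrical box.
; Interact casts the player character's InteractableObject to a switch, turns it green, marks it Active and plays a sound.
; It then scans every switch in the level, stopping at the first inactive one.
; When all are active, it turns BP_ElectricalBox green, spawns a point light at a fixed position and flags every switch as BoxCharged.
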(event EventBeginPlay)

(event Collision|EventActorBeginOverlap
  (params (OtherActor :type Actor%20Object%20Reference)))

(event EventTick
  (params (DeltaSeconds :type Float%20%28single-precision%29)))

(event EventInteract
  ;[1 1 1] Get Current Interactable
  (bind _returnvalue (Actor|GetActorOfClass "/Game/FirstPerson/Blueprints/BP_FirstPersonCharacter.BP_FirstPersonCharacter_C"))
  (bind _asbp_electrical_switch (Utilities|Casting|CastToBP_ElectricalSwitch (Variables|/Game/FirstPerson/Blueprints/BP_FirstPersonCharacter.BP_FirstPersonCharacter_C|GetInteractableObject _returnvalue)))
  (bind _outactors (Actor|GetAllActorsOfClass "BP_ElectricalSwitch_C"))
  (for (_ _array_index) _outactors
    _)
  (CallFunction|SetMaterialGreen _asbp_electrical_switch)
  (Audio|PlaySoundatLocation "/Game/Audio/SFX/Switch_Cue.Switch_Cue" (Transformation|GetWorldLocation (Variables|Default|GetCube)) "0, 0, 0" 0.25 1.0 0.0 "/Game/Audio/Music/SA_Speakers.SA_Speakers" 0 0 0)
  (bind _outactors_2 (Actor|GetAllActorsOfClass "BP_ElectricalSwitch_C"))
  (bind _array_element (Utilities|Array|ForEachLoopwithBreak _outactors_2 :!label _label)
    (:LoopBody
      (bind _output_get (Variables|Default|SetbBoxCharged (Variables|BP_ElectricalSwitch_C|GetbActive _array_element)))
      (if (not _output_get)
        (goto _label Break)))
    (:Completed
      (if (Variables|Default|GetbBoxCharged)
        (bind _returnvalue_2 (Actor|GetActorOfClass "/Game/BluePrints/Intactables/BP_ElectricalBox.BP_ElectricalBox_C"))
        (Default|SetMaterialGreen _returnvalue_2)
        (Game|SpawnActorfromClass "/Script/Engine.PointLight" (Math|Conversions|ToTransform(Vector) "-1800.000000,-1050.000000,270.000000") "Undefined" 0 0)
        ;[1 1 1] Make Sure All Switches are Set to Charged
        (bind _array_element_2 (Utilities|Array|ForEachLoopwithBreak _outactors_2)
          (:LoopBody
            (Variables|BP_ElectricalSwitch_C|SetbBoxCharged _array_element_2 true)))))))

(fn ConstructionScript)

(fn SetMaterialGreen
  (Rendering|Material|SetMaterial (Variables|Default|GetCube) 0 "/Game/BluePrints/Intactables/MM_SwitchOn.MM_SwitchOn")
  (Variables|Default|SetbActive true))

(fn SetMaterialRed
  (Rendering|Material|SetMaterial (Variables|Default|GetCube) 0 "/Game/StarterContent/Materials/M_ColorGrid_LowSpec.M_ColorGrid_LowSpec"))