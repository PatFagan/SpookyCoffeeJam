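; BP_CreatureSplineLocker is a scripted creature that crawls along an editable spline path when triggered.
; On BeginPlay the skeletal mesh loops a crawl animation and its audio is paused.
; The MoveCreature event unpauses the audio and plays a timeline, rate-scaled by TimeToComplete, that lerps distance along the spline to set the mesh's world location.
; Only position follows the spline; rotation is never updated.
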(event Custom|MoveCreature
  (bind _spline (Variables|Default|GetSpline))
  (Components|Timeline|SetPlayRate (Variables|Default|GetMoveCreatureTimeline) (/ 1.0 (Variables|Default|GetTimeToComplete)))
  (Class|AudioComponent|SetPaused (Variables|Default|GetAudio) false)
  (bind _move_track (Timeline|MoveCreatureTimeline Play)
    (:Update
      (Transformation|SetWorldLocation (Variables|Default|GetSkeletalMesh) (Spline|GetLocationatDistanceAlongSpline _spline (Math|Float|Lerp 0.0 (Spline|GetSplineLength _spline) _move_track) "World") false false))))

(event EventBeginPlay
  (Components|Animation|PlayAnimation (Variables|Default|GetSkeletalMesh) "/Game/Animations/CreatureCrawl.CreatureCrawl" true)
  (Class|AudioComponent|SetPaused (Variables|Default|GetAudio) true))

(fn ConstructionScript)