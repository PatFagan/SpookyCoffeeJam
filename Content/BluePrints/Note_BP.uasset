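; Interactable note actor that shows a reading widget when the player picks it up.
; Interact toggles reading, hiding the note mesh and blocking move and look input, then reversing both and setting NoteRead on put-down.
; Any key press also closes the widget through PutDownNote, but that path neither restores input nor sets NoteRead.
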(event Custom|TogglePickup
  (bind _returnvalue (Game|GetPlayerController 0))
  (bind _returnvalue_2 (Game|GetPlayerController 0))
  (if (Variables|Default|GetIsReading)
    (CallFunction|PutDownNote)
    (Input|SetIgnoreMoveInput _returnvalue_2 false)
    (Input|SetIgnoreLookInput _returnvalue_2 false)
    (Variables|Default|SetNoteRead true)
    (else
      (CallFunction|PickupNote)
      (Input|SetIgnoreMoveInput _returnvalue true)
      (Input|SetIgnoreLookInput _returnvalue true))))

(event Custom|PickupNote
  (bind _returnvalue (UserInterface|CreateWidget (Variables|Default|GetWidget)))
  (UserInterface|Viewport|AddtoViewport _returnvalue 0)
  (Rendering|SetVisibility (Variables|Default|GetNote) false false)
  (Variables|Default|SetIsReading true))

(event Custom|PutDownNote
  (Utilities|IsValid (stale Custom|PickupNote _returnvalue)
    (:Is%20Valid
      (Widget|RemovefromParent (stale Custom|PickupNote _returnvalue))
      (Rendering|SetVisibility (Variables|Default|GetNote) true false)
      (Variables|Default|SetIsReading false))))

(event EventInteract
  (CallFunction|TogglePickup)
  (Development|PrintString "Hello"))

(event Input|KeyboardEvents|AnyKey
  (params (Key :type Key%20Structure :default "None"))
  (:Pressed
    (CallFunction|PutDownNote)))

(fn ConstructionScript)