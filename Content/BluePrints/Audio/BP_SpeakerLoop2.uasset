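; BP_SpeakerLoop2 is a speaker Blueprint whose audio can be switched on and off during play.
; Its Audio component is paused in both the construction script and BeginPlay.
; The ToggleSpeakers event flips IsON, sets the pause state and prints the speaker status.
; The flag reads inverted: true pauses the audio as "Speaker Off", false resumes it as "Speaker On".
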(event EventToggleSpeakers
  (bind _output_get (Variables|Default|SetIsON? (not (Variables|Default|GetIsON?))))
  (if _output_get
    (Class|AudioComponent|SetPaused (Variables|Default|GetAudio) true)
    (Development|PrintString "Speaker Off")
    (else
      (Class|AudioComponent|SetPaused (Variables|Default|GetAudio) false)
      (Development|PrintString "Speaker On"))))

(event EventBeginPlay
  (Class|AudioComponent|SetPaused (Variables|Default|GetAudio) true))

(fn ConstructionScript
  (Class|AudioComponent|SetPaused (Variables|Default|GetAudio) true))