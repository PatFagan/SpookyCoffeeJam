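; BP_Enemy is an enemy that chases the player's first-person character.
; On BeginPlay it caches the BP_FirstPersonCharacter found with GetActorOfClass and loops the CreatureWalking animation directly on its mesh.
; Every Tick it reissues SimpleMoveToActor on its controller toward that cached player.
; The overlap event is empty, so contact with the player has no effect in this graph.
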(event EventBeginPlay
  (bind _returnvalue (Actor|GetActorOfClass "/Game/FirstPerson/Blueprints/BP_FirstPersonCharacter.BP_FirstPersonCharacter_C"))
  (Variables|Default|SetPlayerReference _returnvalue)
  (Components|Animation|PlayAnimation (Variables|Character|GetMesh) "/Game/Animations/CreatureWalking.CreatureWalking" true))

(event Collision|EventActorBeginOverlap
  (params (OtherActor :type Actor%20Object%20Reference)))

(event EventTick
  (params (DeltaSeconds :type Float%20%28single-precision%29))
  (AI|Navigation|SimpleMovetoActor (Pawn|GetController) (Variables|Default|GetPlayerReference)))

(fn ConstructionScript)