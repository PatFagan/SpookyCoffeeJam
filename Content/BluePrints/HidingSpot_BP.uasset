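; Hiding spot, such as a locker, that the player enters and exits through an Interact event.
; Box overlap with the first-person character opens a gate and enables input; leaving closes it, disables input and stops movement.
; Interact swings the door via timeline, plays a shuffle sound and toggles character visibility, collision, look input and blended view target.
; A short delay then re-enables input and reopens the gate.
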(event OnComponentBeginOverlap(Box)
  (params (OverlappedComponent :type Primitive%20Component%20Object%20Reference) (OtherActor :type Actor%20Object%20Reference) (OtherComp :type Primitive%20Component%20Object%20Reference) (OtherBodyIndex :type Integer) (bFromSweep :type Boolean) (SweepResult :type Hit%20Result%20Structure%20%28by%20ref%29))
  ;[1 1 1] In And Out of Locker
  (bind _asbp_first_person_character (Utilities|Casting|CastToBP_FirstPersonCharacter OtherActor))
  (Variables|Default|SetCharacterRef _asbp_first_person_character)
  (Input|EnableInput (Game|GetPlayerController 0))
  (Utilities|FlowControl|Gate true) ; enters at Open
)

(event OnComponentEndOverlap(Box)
  (params (OverlappedComponent :type Primitive%20Component%20Object%20Reference) (OtherActor :type Actor%20Object%20Reference) (OtherComp :type Primitive%20Component%20Object%20Reference) (OtherBodyIndex :type Integer))
  (bind _returnvalue (Game|GetPlayerController 0))
  ;[1 1 1] In And Out of Locker
  (bind _asbp_first_person_character (Utilities|Casting|CastToBP_FirstPersonCharacter OtherActor))
  (Components|Movement|StopMovementImmediately (Variables|/Script/Engine.Character|GetCharacterMovement _asbp_first_person_character))
  (Input|DisableInput _returnvalue)
  (Utilities|FlowControl|Gate true) ; enters at Close
)

(event EventInteract
  ;[1 1 1] In And Out of Locker
  (Utilities|FlowControl|Gate true :!label _label
    (:Exit
      (Utilities|FlowControl|Sequence
        (:then_0
          (CallFunction|ToggleHide)
          (Audio|PlaySoundatLocation "/Game/Audio/SFX/HidingShuffle.HidingShuffle" (Transformation|GetWorldLocation (Variables|Default|GetDoor)) "0, 0, 0" 1.0 1.0 0.0 0 0 0 0)
          (Utilities|FlowControl|Delay 0.2)
          (Input|EnableInput (Game|GetPlayerController 0))
          (goto _label Open))
        (:then_1
          (bind _door (Timeline|Open/Close_T PlayFromStart)
            (:Update
              (Transformation|SetRelativeRotation (Variables|Default|GetDoor) (Math|Rotator|MakeRotator 0.0 0.0 (Math|Float|Lerp (Variables|Default|GetCloseAngle) (Variables|Default|GetOpenAngle) _door)) false false))))))))

(fn ConstructionScript)

(fn ToggleHide
  (bind _returnvalue (Game|GetPlayerController 0))
  (bind _characterref (Variables|Default|GetCharacterRef))
  (if (Variables|Default|GetIsHiding)
    (Variables|Default|SetIsHiding false)
    (Rendering|SetActorHiddenInGame _characterref false)
    (Collision|SetActorEnableCollision _characterref true)
    (Input|SetIgnoreLookInput _returnvalue false)
    (Game|Player|SetViewTargetwithBlend _returnvalue _characterref 0.8 "VTBlend_Linear" 0.0 false)
    (else
      (Variables|Default|SetIsHiding true)
      (Rendering|SetActorHiddenInGame _characterref true)
      (Collision|SetActorEnableCollision _characterref false)
      (Input|SetIgnoreLookInput _returnvalue true)
      (Game|Player|SetViewTargetwithBlend _returnvalue self 0.8 "VTBlend_Linear" 0.0 false))))