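; Monster actor that crawls along a spline path using a looping crawl animation started on BeginPlay.
; Each Tick advances a distance by Speed and samples the spline's local transform to set the skeletal mesh's relative transform with sweep.
; Fixed height and yaw offsets adjust the mesh placement on the path.
; The distance never wraps or resets, and is printed every frame for debugging.
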(event EventBeginPlay
  (Components|Animation|PlayAnimation (Variables|Default|GetSkeletalMesh) "/Game/Animations/CreatureCrawl.CreatureCrawl" true))

(event EventTick
  (params (DeltaSeconds :type Float%20%28single-precision%29))
  ;[1 1 1] Spline
  (bind _output_get (Variables|Default|SetDistanceAlongSpline (+ (* DeltaSeconds (Variables|Default|GetSpeed)) (Variables|Default|GetDistanceAlongSpline))))
  (Transformation|SetRelativeTransform (Variables|Default|GetSkeletalMesh) (Math|Transform|MakeTransform (Math|Vector|MakeVector (.x (.location (Spline|GetTransformatDistanceAlongSpline (Variables|Default|GetSpline1) _output_get "Local" false))) (.y (.location (Spline|GetTransformatDistanceAlongSpline (Variables|Default|GetSpline1) _output_get "Local" false))) (+ (.z (.location (Spline|GetTransformatDistanceAlongSpline (Variables|Default|GetSpline1) _output_get "Local" false))) -89.0)) (Math|Rotator|MakeRotator (.roll (.rotation (Spline|GetTransformatDistanceAlongSpline (Variables|Default|GetSpline1) _output_get "Local" false))) (.pitch (.rotation (Spline|GetTransformatDistanceAlongSpline (Variables|Default|GetSpline1) _output_get "Local" false))) (+ (.yaw (.rotation (Spline|GetTransformatDistanceAlongSpline (Variables|Default|GetSpline1) _output_get "Local" false))) -9e+01)) "1.000000,1.000000,1.000000") true false)
  (Development|PrintString (Utilities|String|ToString(Float) (Variables|Default|GetDistanceAlongSpline))))

(fn ConstructionScript)