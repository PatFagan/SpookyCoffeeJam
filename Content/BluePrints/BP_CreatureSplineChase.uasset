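; Creature actor that chases along a spline and teleports the first-person player to a fixed world spot on contact.
; It loops a walk animation from BeginPlay; MoveCreature plays a timeline, rate-scaled by TimeToComplete, that moves the skeletal mesh along the spline with a yaw correction.
; Overlapping Box2 waits one second, then casts to BP_FirstPersonCharacter and resets its transform to the hardcoded location and facing.
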(event OnComponentBeginOverlap(Box2)
  (params (OverlappedComponent :type Primitive%20Component%20Object%20Reference) (OtherActor :type Actor%20Object%20Reference) (OtherComp :type Primitive%20Component%20Object%20Reference) (OtherBodyIndex :type Integer) (bFromSweep :type Boolean) (SweepResult :type Hit%20Result%20Structure%20%28by%20ref%29))
  ;[1 1 1] Call the hit player effect
  (Utilities|FlowControl|Delay 1.0)
  (bind _asbp_first_person_character (Utilities|Casting|CastToBP_FirstPersonCharacter OtherActor))
  (Transformation|SetWorldTransform (Variables|/Script/Engine.Actor|GetRootComponent _asbp_first_person_character) (Math|Transform|MakeTransform (Math|Vector|MakeVector -3605.0 -8715.0 2.1e+02) (Math|Rotator|MakeRotator 0.0 0.0 9e+01) "1.000000,1.000000,1.000000") false false))

(event Custom|MoveCreature
  (bind _spline (Variables|Default|GetSpline))
  (Components|Timeline|SetPlayRate (Variables|Default|GetMoveCreatureTimeline) (/ 1.0 (Variables|Default|GetTimeToComplete)))
  (bind _move_track (Timeline|MoveCreatureTimeline Play)
    (:Update
      (Transformation|SetWorldTransform (Variables|Default|GetSkeletalMesh) (Math|Transform|MakeTransform (Math|Vector|MakeVector (.x (.location (Spline|GetTransformatDistanceAlongSpline _spline (Math|Float|Lerp 0.0 (Spline|GetSplineLength _spline) _move_track) "World" false))) (.y (.location (Spline|GetTransformatDistanceAlongSpline _spline (Math|Float|Lerp 0.0 (Spline|GetSplineLength _spline) _move_track) "World" false))) (.z (.location (Spline|GetTransformatDistanceAlongSpline _spline (Math|Float|Lerp 0.0 (Spline|GetSplineLength _spline) _move_track) "World" false)))) (Math|Rotator|MakeRotator (.roll (.rotation (Spline|GetTransformatDistanceAlongSpline _spline (Math|Float|Lerp 0.0 (Spline|GetSplineLength _spline) _move_track) "World" false))) (.pitch (.rotation (Spline|GetTransformatDistanceAlongSpline _spline (Math|Float|Lerp 0.0 (Spline|GetSplineLength _spline) _move_track) "World" false))) (+ (.yaw (.rotation (Spline|GetTransformatDistanceAlongSpline _spline (Math|Float|Lerp 0.0 (Spline|GetSplineLength _spline) _move_track) "World" false))) -9e+01)) "1.000000,1.000000,1.000000") false false))))

(event EventBeginPlay
  (Components|Animation|PlayAnimation (Variables|Default|GetSkeletalMesh) "/Game/Animations/CreatureWalking.CreatureWalking" true))

(fn ConstructionScript)